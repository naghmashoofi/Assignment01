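; BP_SpawnManager is a spawner actor that scatters random collectibles across an area when play begins.
; On BeginPlay it loops SpawnCount times, picking a random class from CollectibleClasses on each pass.
; Each spawn gets a random X and Y within the configured min and max bounds, takes the manager's own Z, and always spawns regardless of collision.
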(event `self.ReceiveBeginPlay`
  ; Spawn random collectibles at BeginPlay
  (for _ (range (`self.SpawnCount`))
    (`|SpawnActorFromClass` (`KismetArrayLibrary.Array_Random` (`self.CollectibleClasses`)) (`KismetMathLibrary.MakeTransform` (`KismetMathLibrary.MakeVector` (`KismetMathLibrary.RandomFloatInRange` (`self.SpawnMinX`) (`self.SpawnMaxX`)) (`KismetMathLibrary.RandomFloatInRange` (`self.SpawnMinY`) (`self.SpawnMaxY`)) (.z (`self.K2_GetActorLocation`)))) "AlwaysSpawn" "MultiplyWithRoot" null null)))

(fn `UserConstructionScript`)