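; BP_Door is a door actor that swings open about its DoorPivot.
; InteractionTrigger overlaps register the door as NearbyDoor on BP_ThirdPersonCharacter, clearing it on exit only if it still points to this door.
; The OpenDoor event plays a timeline that scales OpenAngle by its alpha to set the pivot's relative yaw, with no closing logic.
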(event `OpenDoor`
  ; Animate door opening
  (bind (_direction _openalpha) (`Timeline|TL_OpenDoor`)
    (:`Update`
      (`SceneComponent.K2_SetRelativeRotation` (`self.DoorPivot`) (`KismetMathLibrary.MakeRotator` 0.0 0.0 (* _openalpha (`self.OpenAngle`))) false false))))

(event `self.InteractionTrigger.OnComponentEndOverlap`
  (params (OverlappedComponent :type "PrimitiveComponent Object Reference") (OtherActor :type "Actor Object Reference") (OtherComp :type "PrimitiveComponent Object Reference") (OtherBodyIndex :type Integer))
  ; clear nearby door on exit
  (bind _asbp_third_person_character (cast `/Game/ThirdPerson/Blueprints/BP_ThirdPersonCharacter` OtherActor))
  (if (== (`/Game/ThirdPerson/Blueprints/BP_ThirdPersonCharacter.NearbyDoor` _asbp_third_person_character) self)
    (set `/Game/ThirdPerson/Blueprints/BP_ThirdPersonCharacter.NearbyDoor` null _asbp_third_person_character)))

(event `self.InteractionTrigger.OnComponentBeginOverlap`
  (params (OverlappedComponent :type "PrimitiveComponent Object Reference") (OtherActor :type "Actor Object Reference") (OtherComp :type "PrimitiveComponent Object Reference") (OtherBodyIndex :type Integer) (bFromSweep :type Boolean) (SweepResult :type "HitResult Structure (by ref)"))
  ; Register nearby door
  (bind _asbp_third_person_character (cast `/Game/ThirdPerson/Blueprints/BP_ThirdPersonCharacter` OtherActor))
  (set `/Game/ThirdPerson/Blueprints/BP_ThirdPersonCharacter.NearbyDoor` self _asbp_third_person_character))

(fn `UserConstructionScript`)